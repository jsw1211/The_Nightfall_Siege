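; BP_DamageActor is a floating damage number actor that shows a damage value in the world and then removes itself.
; On BeginPlay it passes its Damage value to the WBP_DamageText widget in its widget component.
; A MoveUp timeline raises the actor from its spawn location while fading the red text's alpha in proportion to height, then destroys the actor when finished.
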(event `self.ReceiveBeginPlay`
  (bind _aswbp_damage_text (cast `/Game/BP/WBP_DamageText` (`WidgetComponent.GetUserWidgetObject` (`self.Widget`))))
  (set `self.DamageWidget` _aswbp_damage_text)
  (`/Game/BP/WBP_DamageText.SetDamage` _aswbp_damage_text (`self.Damage`))
  (set `self.StartLocation` (`self.K2_GetActorLocation`))
  (bind (_direction _height) (`Timeline|MoveUp` :!via `PlayFromStart`)
    (:`Update`
      (`self.K2_SetActorLocation` (`KismetMathLibrary.MakeVector` (.x (`self.StartLocation`)) (.y (`self.StartLocation`)) (+ _height (.z (`self.StartLocation`)))))
      (`TextBlock.SetColorAndOpacity` (`/Game/BP/WBP_DamageText.DamageText` (`self.DamageWidget`)) (make `SlateColor` (make `LinearColor` 1.0 0.0 0.0 (- 1.0 (/ _height 80.0))))))
    (:`Finished`
      (`self.K2_DestroyActor`))))

(fn `UserConstructionScript`)